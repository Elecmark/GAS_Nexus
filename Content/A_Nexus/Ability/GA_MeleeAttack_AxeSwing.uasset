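; Gameplay ability for an axe swing melee attack that requires an equipped weapon from the avatar's WeaponsManagerComponent, ending immediately without one.
; It plays the swing montage and ends when the montage completes, is interrupted or is cancelled.
; On the authority, HitScan Start and End gameplay events open and close the weapon's hit scan, passing it an instant damage spec with a SetByCaller magnitude.
; Ending the ability also stops the hit scan.
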(event Ability|EventActivateAbility
  (bind _returnvalue (Ability|GetAvatarActorfromActorInfo))
  (bind _returnvalue_2 (Actor|GetComponentbyClass _returnvalue "/Game/A_Nexus/Weapons/WeaponsManagerComponent.WeaponsManagerComponent_C"))
  (Utilities|IsValid _returnvalue_2
    (:Is%20Valid
      (bind _equipedweapon (Variables|/Game/A_Nexus/Weapons/WeaponsManagerComponent.WeaponsManagerComponent_C|GetEquipedWeapon _returnvalue_2)
        (:then
          (Variables|Default|SetEquiped%20Weapon _equipedweapon)
          (|PlayMontageandWaitProxy "None" "/Game/A_Nexus/Animations/Axe/Am_AxeMelee_AxeSwing.Am_AxeMelee_AxeSwing" 1.0 "None" true 1.0 0.0 true
            (:then
              (Ability|HasAuthority
                (:True
                  (Ability|Tasks|WaitGameplayEvent "(TagName=\"Event.HitScan.Start\")" 0
                    (:then
                      (Ability|Tasks|WaitGameplayEvent "(TagName=\"Event.HitScan.End\")" 0
                        (:EventReceived
                          (bind _equiped_weapon (Variables|Default|GetEquiped%20Weapon)
                            (:then
                              (Default|HitScanEnd _equiped_weapon))
                            (:else)))))
                    (:EventReceived
                      (bind _equiped_weapon_2 (Variables|Default|GetEquiped%20Weapon)
                        (:then
                          (bind _returnvalue_3 (Ability|GameplayEffect|AssignTagSetbyCallerMagnitude (Ability|MakeOutgoingGameplayEffectSpec "/Game/A_Nexus/Effect/GE_DamageInstant.GE_DamageInstant_C") "(TagName=\"Data.Damage\")" -3e+01))
                          (Default|HitScanStart _equiped_weapon_2 _returnvalue_3))
                        (:else)))))))
            (:OnCompleted
              (Ability|EndAbility :!label _label))
            (:OnInterrupted
              (goto _label))
            (:OnCancelled
              (goto _label))))
        (:else
          (goto _label))))
    (:Is%20Not%20Valid
      (goto _label))))

(event Ability|EventOnEndAbility
  (params (bWasCancelled :type Boolean))
  (bind _equiped_weapon (Variables|Default|GetEquiped%20Weapon)
    (:then
      (Default|HitScanEnd _equiped_weapon))
    (:else)))