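; Base Gameplay Ability that turns stacked debuffs into a status effect on the target, configured by a StatusEffectDA data asset.
; On activation it listens for effects the owner applies to targets, checking each for the debuff tag and maximum stack count.
; When both match, it builds the status effect spec with the configured duration and applies it to that target.
; ModifyEffectSpecBeforeApplication is a pass-through hook for adjusting the spec before application.
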(event Ability|EventActivateAbility
  (bind (_asynctaskproxy _target _spechandle _activehandle) (Ability|Tasks|WaitGameplayEffectAppliedToTarget :OptionalExternalOwner 0)
    (:OnApplied
      (Utilities|IsValid (Ability|GameplayEffect|GetGameplayEffectfromActiveEffectHandle _activehandle)
        (:Is%20Valid
          (if (GameplayTags|HasMatchingGameplayTag (Ability|GameplayEffect|GetGameplayEffectfromActiveEffectHandle _activehandle) (Variables|/Game/A_Nexus/Data/PrimaryDataAsset/PDA_StatusEffect.PDA_StatusEffect_C|GetDebuffTag (Variables|Default|GetStatusEffectDA)))
            (bind _returnvalue (Ability|GameplayEffect|GetActiveGameplayEffectStackCount _activehandle))
            (if (>= _returnvalue (Variables|/Game/A_Nexus/Data/PrimaryDataAsset/PDA_StatusEffect.PDA_StatusEffect_C|GetMaxStackCount (Variables|Default|GetStatusEffectDA)))
              (bind _returnvalue_2 (Ability|GameplayEffect|SetDuration (Ability|MakeOutgoingGameplayEffectSpec (Variables|/Game/A_Nexus/Data/PrimaryDataAsset/PDA_StatusEffect.PDA_StatusEffect_C|GetStatusEffectToApply (Variables|Default|GetStatusEffectDA))) (Variables|/Game/A_Nexus/Data/PrimaryDataAsset/PDA_StatusEffect.PDA_StatusEffect_C|GetStatusDuration (Variables|Default|GetStatusEffectDA))))
              (bind _specout (CallFunction|ModifyEffectSpecBeforeApplication _returnvalue_2))
              (GameplayEffects|ApplyGameplayEffectSpecToTarget _specout (Ability|TargetData|AbilityTargetDatafromActor _target)))))))))

(fn ModifyEffectSpecBeforeApplication
  (params (SpecIn :type Gameplay%20Effect%20Spec%20Handle%20Structure))
  (return SpecIn))