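; Base melee attack Gameplay Ability that plays an attack montage and drives hit scanning on the avatar's equipped weapon.
; On authority, HitScan Start and End gameplay events toggle the weapon's scan, passing it a SetByCaller damage spec scaled by ability level.
; The ability commits only when the montage completes or is interrupted or cancelled, and ending it stops the scan.
; MontageStarted is an empty hook.
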(event Custom|MontageStarted)

(event Custom|HandleHitScanStart
  ;[0.15 0.15 0.15 0.5] HitScan Event
  (bind _equipedweapon (Variables|默认|GetEquipedWeapon)
    (:then
      (bind _returnvalue (Ability|GameplayEffect|AssignTagSetbyCallerMagnitude (Ability|MakeOutgoingGameplayEffectSpec (Variables|GameplayEffect|GetDamageEffectClass)) "(TagName=\"Data.Damage\")" (|({F6002A73-4263-FE31-E9BF-8A975922CD4B}+(({F6002A73-4263-FE31-E9BF-8A975922CD4B}*0.250000)*(AbilityLevel-1))) (Math|Conversions|ToFloat(Integer) (Ability|GetAbilityLevel)))))
      (Default|HitScanStart _equipedweapon _returnvalue))
    (:else)))

(event Custom|HandleHitScanEnd
  ;[0.15 0.15 0.15 0.5] HitScan Event
  (bind _equipedweapon (Variables|默认|GetEquipedWeapon)
    (:then
      (Default|HitScanEnd _equipedweapon))
    (:else)))

(event Ability|EventActivateAbility
  (bind _returnvalue (Ability|GetAvatarActorfromActorInfo))
  (bind _returnvalue_2 (Actor|GetComponentbyClass _returnvalue "/Game/A_Nexus/Weapons/WeaponsManagerComponent.WeaponsManagerComponent_C"))
  (Utilities|IsValid _returnvalue_2
    (:Is%20Valid
      (bind _equipedweapon (Variables|/Game/A_Nexus/Weapons/WeaponsManagerComponent.WeaponsManagerComponent_C|GetEquipedWeapon _returnvalue_2)
        (:then
          (Variables|默认|SetEquipedWeapon _equipedweapon)
          (bind _attackmontage (Variables|动画|GetAttackMontage)
            (:then
              (|PlayMontageandWaitProxy "None" _attackmontage 1.0 "None" true 1.0 0.0 true
                (:then
                  (CallFunction|MontageStarted)
                  (Ability|HasAuthority
                    (:True
                      (Ability|Tasks|WaitGameplayEvent "(TagName=\"Event.HitScan.Start\")" 0
                        (:then
                          (Ability|Tasks|WaitGameplayEvent "(TagName=\"Event.HitScan.End\")" 0
                            (:EventReceived
                              (CallFunction|HandleHitScanEnd))))
                        (:EventReceived
                          (CallFunction|HandleHitScanStart))))))
                (:OnCompleted
                  (Ability|CommitAbility :!label _label)
                  (Ability|EndAbility))
                (:OnInterrupted
                  (goto _label))
                (:OnCancelled
                  (goto _label))))
            (:else)))
        (:else
          (goto _label))))
    (:Is%20Not%20Valid
      (goto _label))))

(event Ability|EventOnEndAbility
  (params (bWasCancelled :type Boolean))
  (CallFunction|HandleHitScanEnd))