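; Staff gameplay ability that calls a lightning bolt onto a ground area, damaging pawns in a radius that scales with ability level.
; It aims at the ground under a preset attack target, otherwise player controllers pick a spot with a decal target actor and looping montage.
; On commit it shows an indicator cue, waits for the montage trigger event, then applies server-side SetByCaller damage via sphere trace.
; Pressing input again cancels before release.
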(event Custom|StartTargeting
  ;[0.15 0.15 0.15 0.5 36] Aim
  (if (Class|NexusGameplayAbility|HasPC)
    (CallFunction|LoopTargetingAnimation)
    (Variables|Default|SetbWaitingTargetData true)
    (GameplayCue|AddGameplayCue :GameplayCueTag "(TagName=\"GameplayCue.TargetingCamera\")")
    (bind _data (|WaitTargetData :ConfirmationType "UserConfirmed" :Class "/Game/A_Nexus/TargettingActors/GATargetActor_GroundTrace_Decal.GATargetActor_GroundTrace_Decal_C" :DecalSize (* (|(({F2AD18E2-4CF5-D748-9018-32AE1C71324E}*(AbilityLevel+1))/2) (Math|Conversions|ToFloat(Integer) (Ability|GetAbilityLevel))) 2.0) :DecalMaterial "/Game/Decals/Decal_AOE.Decal_AOE" :MaxRange 1e+03 :StartLocation (Class|GameplayAbility|MakeTargetLocationInfofromOwnerSkeletalMeshComponent "S_Staff") :ReticleClass 0)
      (:ValidData
        (Variables|Default|SetbWaitingTargetData false)
        (Variables|Default|SetComfirmedAOELocation (.Location (Collision|BreakHitResult (Ability|TargetData|GetHitResultfromTargetData _data))))
        (CallFunction|ConfirmStrike)))
    (else
      (Ability|EndAbility))))

(event Custom|AOEDamage
  (bind _comfirmedaoelocation (Variables|Default|GetComfirmedAOELocation))
  ;[0.15 0.15 0.15 0.5 36] Attack
  (Ability|HasAuthority
    (:True
      (bind _outhits (Collision|MultiSphereTraceForObjects _comfirmedaoelocation _comfirmedaoelocation (|(({F2AD18E2-4CF5-D748-9018-32AE1C71324E}*(AbilityLevel+1))/2) (Math|Conversions|ToFloat(Integer) (Ability|GetAbilityLevel))) (Utilities|Array|MakeArray "ObjectTypeQuery3") false (Utilities|Array|MakeArray (Ability|GetAvatarActorfromActorInfo)) "None"))
      (Utilities|Array|Clear (Variables|Default|GetHitActors))
      (bind _array_element (Utilities|Array|ForEachLoopwithBreak _outhits)
        (:LoopBody
          (if (not (Utilities|Array|ContainsItem (Variables|Default|GetHitActors) (.HitActor (Collision|BreakHitResult _array_element))))
            (Utilities|Array|AddUnique (Variables|Default|GetHitActors) (.HitActor (Collision|BreakHitResult _array_element)))
            (Utilities|IsValid (Ability|GetAbilitySystemComponent (.HitActor (Collision|BreakHitResult _array_element)))
              (:Is%20Valid
                (bind _returnvalue (Ability|GameplayEffect|AssignTagSetbyCallerMagnitude (Ability|MakeOutgoingGameplayEffectSpec "/Game/A_Nexus/Effect/GE_DamageInstant.GE_DamageInstant_C") "(TagName=\"Data.Damage\")" (Variables|Default|GetDamageMagnitude)))
                (GameplayEffects|ApplyGameplayEffectSpecToTarget (Ability|GetAbilitySystemComponent (Ability|GetAvatarActorfromActorInfo)) _returnvalue (Ability|GetAbilitySystemComponent (.HitActor (Collision|BreakHitResult _array_element))))))))))))

(event Custom|ConfirmStrike
  ;[0.15 0.15 0.15 0.5 36] Attack
  (bind _returnvalue (Ability|CommitAbility))
  (if _returnvalue
    (Class|GameplayAbility|AddGameplayCuewithParams "(TagName=\"GameplayCue.AOEIndicator\")" (Ability|GameplayCue|MakeGameplayCueParameters :RawMagnitude (* (|(({F2AD18E2-4CF5-D748-9018-32AE1C71324E}*(AbilityLevel+1))/2) (Math|Conversions|ToFloat(Integer) (Ability|GetAbilityLevel))) 2.0) :Location (Variables|Default|GetComfirmedAOELocation) :Instigator (Ability|GetAvatarActorfromActorInfo)) true)
    (|PlayMontageandWaitProxy "None" "/Game/A_Nexus/Animations/Staff/AM_AOE_Trigger.AM_AOE_Trigger" 1.0 "None" true 1.0 0.0 false
      (:then
        (Variables|Default|SetbRelease true)
        (Ability|Tasks|WaitGameplayEvent "(TagName=\"Event.Montage.Trigger\")" 0
          (:EventReceived
            (Class|GameplayAbility|ExecuteGameplayCuewithParams "(TagName=\"GameplayCue.LightningBolt\")" (Ability|GameplayCue|MakeGameplayCueParameters :Location (Variables|Default|GetComfirmedAOELocation)))
            (Utilities|FlowControl|Delay 0.2)
            (CallFunction|AOEDamage)
            (GameplayCue|RemoveGameplayCue "(TagName=\"GameplayCue.AOEIndicator\")"))))
      (:OnCompleted
        (Ability|EndAbility :!label _label))
      (:OnInterrupted
        (goto _label)))
    (else
      (Ability|EndAbility))))

(event Custom|LoopTargetingAnimation
  ;[0.15 0.15 0.15 0.5 36] Aim
  (|PlayMontageandWaitProxy "None" "/Game/A_Nexus/Animations/Staff/AM_AOE_Targeting.AM_AOE_Targeting" 1.0 "None" true 1.0 0.0 false
    (:then
      (Variables|Default|SetbRelease false))
    (:OnBlendOut
      (if (Variables|Default|GetbWaitingTargetData)
        (CallFunction|LoopTargetingAnimation)))
    (:OnInterrupted
      (if (Variables|Default|GetbWaitingTargetData)
        (Ability|EndAbility)))))

(event Custom|WaitCancelInput
  ;[0.15 0.15 0.15 0.5 36] Attack
  (Ability|Tasks|WaitInputPress false
    (:OnPress
      (if (not (Variables|Default|GetbRelease))
        (Ability|EndAbility)))))

(event Ability|EventActivateAbility
  ;[0.15 0.15 0.15 0.5 36] Aim
  (CallFunction|WaitCancelInput)
  (bind _attacktarget (Class|BPITargeting|GetAttackTarget(Message) (Ability|GetAvatarActorfromActorInfo)))
  (Utilities|IsValid _attacktarget
    (:Is%20Valid
      (Variables|Default|SetComfirmedAOELocation (.TargetLocation (CallFunction|GetTargetGroundLocation _attacktarget)))
      (CallFunction|ConfirmStrike))
    (:Is%20Not%20Valid
      (CallFunction|StartTargeting))))

(fn GetTargetGroundLocation
  (params (AttackTarget :type Actor%20Object%20Reference))
  (bind _returnvalue (Transformation|GetActorLocation AttackTarget))
  (bind (_outhit _returnvalue_2) (Collision|LineTraceByChannel _returnvalue (- _returnvalue "0.000000,0.000000,100000.000000") "TraceTypeQuery1" false (Utilities|Array|MakeArray AttackTarget) "None"))
  (return (.Location (Collision|BreakHitResult _outhit)) _returnvalue_2))