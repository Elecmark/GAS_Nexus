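; Base staff weapon ability that plays a shoot montage and fires a projectile when the Event.ShootProjectile gameplay event arrives.
; It aims at the avatar's attack target, falling back to an instant line-trace target for player-controlled avatars and ending otherwise.
; The projectile spawns only on authority at the equipped weapon's spawn point or actor location, carrying a SetByCaller damage effect spec.
; The ability also ends when the montage completes, is interrupted or is cancelled.
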(event Custom|Shoot%20Projectile
  (params (TargetLocation :type Vector))
  (bind _returnvalue (Ability|GameplayEffect|AssignTagSetbyCallerMagnitude (Ability|MakeOutgoingGameplayEffectSpec (Variables|GameplayEffect|GetDamageEffectClass)) "(TagName=\"Data.Damage\")" (Variables|Default|GetDamageMagnitude)))
  (|SpawnActor 0 (CallFunction|GetSpawnLocation) "0, 0, 0" (Variables|Default|GetProjectileClass) true (Variables|Default|GetProjectileSpeed) TargetLocation _returnvalue (.AsPawn (Utilities|Casting|CastToPawn (Ability|GetAvatarActorfromActorInfo)))))

(event Ability|EventActivateAbility
  (|PlayMontageandWaitProxy "None" (Variables|Default|GetShootMontage) 1.0 "None" true 1.0 0.0 true
    (:then
      (Ability|Tasks|WaitGameplayEvent "(TagName=\"Event.ShootProjectile\")" 0
        (:EventReceived
          (bind _attacktarget (Class|BPITargeting|GetAttackTarget(Message) (Ability|GetAvatarActorfromActorInfo)))
          (Utilities|IsValid _attacktarget
            (:Is%20Valid
              (CallFunction|ShootProjectile (Transformation|GetActorLocation _attacktarget)))
            (:Is%20Not%20Valid
              (if (Class|NexusGameplayAbility|HasPC)
                (bind _data (|WaitTargetData :ConfirmationType "Instant" :Class "/Script/GameplayAbilities.GameplayAbilityTargetActor_SingleLineTrace" :TraceProfile "(Name=\"NoCollision\")" :StartLocation (Class|GameplayAbility|MakeTargetLocationInfofromOwnerActor) :ReticleClass 0 :bDebug true)
                  (:ValidData
                    (CallFunction|ShootProjectile (Class|AbilitySystemBlueprintLibrary|GetTargetDataEndPoint _data))))
                (else
                  (Ability|EndAbility))))))))
    (:OnCompleted
      (Ability|EndAbility :!label _label))
    (:OnInterrupted
      (goto _label))
    (:OnCancelled
      (goto _label))))

(event Ability|EventOnEndAbility
  (params (bWasCancelled :type Boolean)))

(fn GetSpawnLocation
  (bind _returnvalue (Ability|GetAvatarActorfromActorInfo))
  (bind _returnvalue_2 (Actor|GetComponentbyClass _returnvalue "/Game/A_Nexus/Weapons/WeaponsManagerComponent.WeaponsManagerComponent_C"))
  (Utilities|IsValid _returnvalue_2
    (:Is%20Valid
      (bind _equipedweapon (Variables|/Game/A_Nexus/Weapons/WeaponsManagerComponent.WeaponsManagerComponent_C|GetEquipedWeapon _returnvalue_2)
        (:then
          (bind _location (Default|GetSpawnPointLocation _equipedweapon))
          (if (Utilities|Operators|NotEqual(!=) :A _location)
            (return _location)
            (else
              _)))
        (:else
          _)))
    (:Is%20Not%20Valid
      _))
  (return (Transformation|GetActorLocation (Ability|GetAvatarActorfromActorInfo))))