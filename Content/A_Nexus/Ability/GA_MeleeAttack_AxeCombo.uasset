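; Axe melee combo Gameplay Ability that extends a parent ability's montage and hit-scan attack with timed-input chaining.
; Once the montage starts, gameplay events open and close each combo window and record whether input arrives inside it.
; At window close, timely input increments the combo count, otherwise the ability ends; owners without a player controller always continue.
; Each hit scan scales damage by the combo count before calling the parent handler.
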(event Ability|EventActivateAbility
  (|CallParentFunction)
  (Variables|Default|SetbAlwaysContinueCombo (not (Class|NexusGameplayAbility|HasPC))))

(event Ability|EventOnEndAbility
  (params (bWasCancelled :type Boolean))
  (|CallParentFunction bWasCancelled) ; 此节点被禁用，将不会被调用。\n从引脚连出引线来编译功能。
)

(event EventMontageStarted
  (Variables|Default|SetComboCount 1)
  (Ability|Tasks|WaitGameplayEvent "(TagName=\"Event.ContinueCombo.Start\")" 0
    (:then
      (Ability|Tasks|WaitGameplayEvent "(TagName=\"Event.ContinueCombo.End\")" 0
        (:then
          (Ability|Tasks|WaitGameplayEvent "(TagName=\"Event.ContinueCombo.Input\")" 0
            (:EventReceived
              (Variables|Default|SetbReceivedlnputAtRightTime (Variables|Default|GetbWithinComboWindow)))))
        (:EventReceived
          (Variables|Default|SetbWithinComboWindow false)
          (if (or (Variables|Default|GetbReceivedlnputAtRightTime) (Variables|Default|GetbAlwaysContinueCombo))
            (Math|Integer|IncrementInt (Variables|Default|GetComboCount))
            (else
              (Ability|EndAbility))))))
    (:EventReceived
      (Variables|Default|SetbWithinComboWindow true)
      (Variables|Default|SetbReceivedlnputAtRightTime false))))

(event EventHandleHitScanStart
  (Variables|Default|SetDamageMagnitude (* -25.0 (/ (Variables|Default|GetComboCount) 2)))
  (|CallParentFunction))